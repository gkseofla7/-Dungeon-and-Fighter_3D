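; Fire pickup actor that the ghost knight player can collect into the inventory and use to spawn Fire at the character's drop location.
; Construction Script fills the item struct and mesh from custom variables.
; Trigger overlap toggles the prompt widget and an in-range flag checked by an event bound to the character's PickupItem dispatcher.
; Pickup adds the struct to the HUD inventory, refreshes it, and hides the actor rather than destroying it.
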(event `self.ReceiveBeginPlay`
  (bind _pickuptextreference (`self.PickupTextReference`))
  (bind _iteminfo (`self.ItemInfo`))
  (bind (_item _itemimage _pickuptext) (break `InventoryStruct` _iteminfo))
  ;[1 1 1] Event Begin Play
  (bind _returnvalue (`|CreateWidget` "/Game/UI/PickupText.PickupText_C"))
  (set `self.PickupTextReference` _returnvalue)
  (setmembers `InventoryStruct` :`StructRef` _iteminfo :`Item` self)
  (set `/Game/UI/PickupText.PickupActor` _item _pickuptextreference)
  (set `/Game/UI/PickupText.PickupText` _pickuptext _pickuptextreference)
  (bind _asbp_dfghost_knight (cast `/Game/Blueprints/BP_DFGhostKnight` (`GameplayStatics.GetPlayerCharacter` 0)))
  (bind _output_get (set `self.CharacterReference` _asbp_dfghost_knight))
  (add `/Game/Blueprints/BP_DFGhostKnight.PickupItem` _output_get (delegate `PickupItem_Event_1`)))

(event `PickupItem_Event_1`
  (bind _bp_gamehudreference (`/Game/Blueprints/BP_DFGhostKnight.BP_GameHudReference` (`self.CharacterReference`)))
  ;[1 1 1] Pickup and add items to the inventory refresh it
  (if (and (`self.GetActorEnableCollision`) (`self.IsInRange`))
    (`KismetArrayLibrary.Array_Add` (`DFGameHudWidget.Inventory` _bp_gamehudreference) (`self.ItemInfo`))
    (`Widget.RemoveFromParent` (`self.PickupTextReference`))
    (`self.SetActorHiddenInGame` true)
    (`self.SetActorEnableCollision` false)
    (`/Game/UI/GameHud.RefreshInventory` _bp_gamehudreference)))

(event `self.Trigger.OnComponentBeginOverlap`
  (params (OverlappedComponent :type "PrimitiveComponent Object Reference") (OtherActor :type "Actor Object Reference") (OtherComp :type "PrimitiveComponent Object Reference") (OtherBodyIndex :type Integer) (bFromSweep :type Boolean) (SweepResult :type "HitResult Structure (by ref)"))
  ;[1 1 1] Overlap Trigger Script
  (cast `/Game/Blueprints/BP_DFGhostKnight` OtherActor)
  (`UserWidget.AddToViewport` (`self.PickupTextReference`) 0)
  (set `self.IsInRange` true))

(event `self.Trigger.OnComponentEndOverlap`
  (params (OverlappedComponent :type "PrimitiveComponent Object Reference") (OtherActor :type "Actor Object Reference") (OtherComp :type "PrimitiveComponent Object Reference") (OtherBodyIndex :type Integer))
  ;[1 1 1] Overlap Trigger Script
  (cast `/Game/Blueprints/BP_DFGhostKnight` OtherActor)
  (`Widget.RemoveFromParent` (`self.PickupTextReference`))
  (set `self.IsInRange` false))

(event `/Game/Blueprints/ActioinInterface.UseActioin`
  ;[1 1 1] Use Action
  (`|SpawnActorFromClass` "/Game/StarterContent/Blueprints/Fire.Fire_C" (`SceneComponent.K2_GetComponentToWorld` (`/Game/Blueprints/BP_DFGhostKnight.DropLocation` (`self.CharacterReference`))) "Undefined" "OverrideRootScale" null null))

(fn `UserConstructionScript`
  (setmembers `InventoryStruct` :`StructRef` (`self.ItemInfo`) :`Item` (`self.CharacterReference`) :`ItemImage` (`self.CustomImage`) :`PickupText` (`self.CustomPickupText`) :`ActionText` (`self.CustomActionText`))
  (`StaticMeshComponent.SetStaticMesh` (`self.StaticMesh`) (`self.CustomStaticMesh`)))