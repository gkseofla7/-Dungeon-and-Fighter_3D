(event `self.ReceiveBeginPlay`
  ;[1 1 1] Event Begin Play
  (bind _returnvalue (`|CreateWidget` "/Game/UI/GameHud.GameHud_C"))
  (bind _output_get (set `self.BP_GameHudReference` _returnvalue))
  (`UserWidget.AddToViewport` _output_get 0))

(event `Key|I`
  (params (Key :type "Key Structure"))
  (bind _bp_gamehudreference (`self.BP_GameHudReference`))
  (bind _bp_gamehudreference_2 (`self.BP_GameHudReference`))
  (bind _bp_gamehudreference_3 (`self.BP_GameHudReference`))
  ;[1 1 1] Toggle Inventory Menu
  (:`Pressed`
    (if (and (`DFGameHudWidget.ActivateInventory` _bp_gamehudreference_2) (!= (`self.InventoryDelay`) true))
      (`/Engine/EditorBlueprintResources/StandardMacros.FlipFlop`
        (:`A`
          (set `DFGameHudWidget.InventoryVisible` "Visible" _bp_gamehudreference_2)
          (`self.EnableMouseCursor`)
          (`UserWidget.PlayAnimation` _bp_gamehudreference_3 (`/Game/UI/GameHud.MenuAnim` _bp_gamehudreference_3) 0.0 1 "Forward" 1.0 false)
          (set `self.InventoryDelay` true))
        (:`B`
          (set `self.InventoryDelay` true)
          (`UserWidget.PlayAnimation` _bp_gamehudreference (`/Game/UI/GameHud.MenuAnim` _bp_gamehudreference) 0.0 1 "Reverse" 1.0 false)
          (`KismetSystemLibrary.Delay` 1.0)
          (set `DFGameHudWidget.InventoryVisible` "Hidden" _bp_gamehudreference_2)
          (`self.DisableMouseCursor`)))
      (`KismetSystemLibrary.Delay` 0.5)
      (set `self.InventoryDelay` false))))

(event `Key|E`
  (params (Key :type "Key Structure"))
  ;[1 1 1] Pickup Item
  (:`Pressed`
    (if (< (`KismetArrayLibrary.Array_Length` (`DFGameHudWidget.Inventory` (`self.BP_GameHudReference`))) 5)
      (`self.PickupItem`))))

(event `/Game/Blueprints/ActioinInterface.DropAction`
  (params (`Item To Drop` :type "Actor Object Reference"))
  ;[1 1 1] Drop Items
  (`self.SetActorHiddenInGame` `Item To Drop` false)
  (`self.SetActorEnableCollision` `Item To Drop` true)
  (`self.K2_SetActorTransform` `Item To Drop` (`SceneComponent.K2_GetComponentToWorld` (`self.DropLocation`)) false false))

(fn `EnableMouseCursor`
  (bind _returnvalue (`GameplayStatics.GetPlayerController` 0))
  (`WidgetBlueprintLibrary.SetInputMode_GameAndUIEx` _returnvalue (`self.BP_GameHudReference`))
  (set `PlayerController.bShowMouseCursor` true _returnvalue))

(fn `UserConstructionScript`)